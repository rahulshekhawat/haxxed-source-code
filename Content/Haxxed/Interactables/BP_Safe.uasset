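; BP_Safe is an interactable safe that triggers the end credits.
; BeginPlay sets its description and flags it as requiring su.
; On interact, it enables custom depth rendering on its mesh, waits briefly, then creates the end credits widget.
; It then toggles the game instance's Terminal widget and the credits widget.
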(event EventBeginPlay
  (|CallParentFunction)
  (Variables|Default|SetDescription "This is it!")
  (Variables|Default|SetbRequiresSu true))

(event Collision|EventActorBeginOverlap
  (params (OtherActor :type Actor%20Object%20Reference))
  (|CallParentFunction OtherActor) ; This node is disabled and will not be called.\nDrag off pins to build functionality.
)

(event EventTick
  (params (DeltaSeconds :type Float%20%28single-precision%29))
  (|CallParentFunction DeltaSeconds) ; This node is disabled and will not be called.\nDrag off pins to build functionality.
)

(event EventOnInteract
  (Rendering|SetRenderCustomDepth (Variables|Default|GetStaticMesh) true)
  (Utilities|FlowControl|Delay 3.0)
  (bind _returnvalue (UserInterface|CreateWidget "/Game/Haxxed/UI/WBP_EndCredits.WBP_EndCredits_C"))
  (bind _ashaxxed_game_instance (Utilities|Casting|CastToHaxxedGameInstance (Game|GetGameInstance)))
  (Class|HaxxedWidgetBase|ToggleWidget (Variables|/Script/Haxxed.HaxxedGameInstance|GetTerminal _ashaxxed_game_instance))
  (Class|HaxxedWidgetBase|ToggleWidget _returnvalue))

(fn ConstructionScript
  (|CallParentFunction))