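; BP_Door_Locked is an interactable door that requires su access and guards the player's goal.
; BeginPlay runs the parent logic, then sets the description and the RequiresSu flag.
; OnInteract snaps the door to a fixed rotation and spawns a BP_TargetPoint at a hard-coded location, named "SUPERSECRETDOCS".
; The su check is not in this graph, which only sets the flag.
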(event EventBeginPlay
  (|CallParentFunction)
  (Variables|Default|SetDescription "A wooden-textured, quaintly scaled door with SU written indistinctly on it. Behind this, is your goal.")
  (Variables|Default|SetbRequiresSu true))

(event Collision|EventActorBeginOverlap
  (params (OtherActor :type Actor%20Object%20Reference))
  (|CallParentFunction OtherActor) ; This node is disabled and will not be called.\nDrag off pins to build functionality.
)

(event EventTick
  (params (DeltaSeconds :type Float%20%28single-precision%29))
  (|CallParentFunction DeltaSeconds) ; This node is disabled and will not be called.\nDrag off pins to build functionality.
)

(event EventOnInteract
  (Transformation|SetActorRotation "0,-90.000000, 0")
  (bind _returnvalue (Game|SpawnActorfromClass "/Game/Haxxed/Interactables/BP_TargetPoint.BP_TargetPoint_C" (Math|Transform|MakeTransform "-1790.000000,870.000000,290.000000") "Undefined" 0 0))
  (Variables|/Script/Haxxed.HaxxedTargetPoint|SetInGameName _returnvalue "SUPERSECRETDOCS"))

(fn ConstructionScript
  (|CallParentFunction))